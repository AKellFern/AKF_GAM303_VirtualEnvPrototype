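; BP_WeightedBox is an interactable physics box that the player can pick up and drop through interface events.
; On interact, if the player is not already holding something, it sets IsHolding, disables physics and collision on HeldMesh, and attaches the mesh to the player's Arrow1.
; On drop, it calls DetachFromActor and restores collision and physics, without clearing IsHolding itself.
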(event `/Game/Interfaces/Interface_Interact.INT_Interact`
  (params (PlayerRef :type "/Game/Player/BP_PlayerChar Object Reference"))
  (bind _heldmesh (`self.HeldMesh`))
  (if (not (`/Game/Player/BP_PlayerChar.isHolding?` PlayerRef))
    (set `/Game/Player/BP_PlayerChar.isHolding?` true PlayerRef)
    (`PrimitiveComponent.SetSimulatePhysics` _heldmesh false)
    (`PrimitiveComponent.SetCollisionEnabled` _heldmesh "NoCollision")
    (`SceneComponent.K2_AttachToComponent` _heldmesh (`/Game/Player/BP_PlayerChar.Arrow1` PlayerRef) "None" "SnapToTarget" "KeepRelative" "KeepRelative" true)))

(event `/Game/Interfaces/Interface_Interact.INT_Drop`
  (bind _heldmesh (`self.HeldMesh`))
  (`self.K2_DetachFromActor` "KeepWorld" "KeepWorld" "KeepWorld")
  (`PrimitiveComponent.SetCollisionEnabled` _heldmesh "QueryAndPhysics")
  (`PrimitiveComponent.SetSimulatePhysics` _heldmesh true))

(fn `UserConstructionScript`)